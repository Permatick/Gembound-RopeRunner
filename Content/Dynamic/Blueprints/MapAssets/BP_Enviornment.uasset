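; Environment segment that self-populates and triggers extension of the level as the player moves through it.
; The construction script runs SpawnEnv, adding child actor components at eight Sp marker transforms, four with a random seven-way branch and four fixed.
; A player overlap on the Box calls ExtendEnv on BP_GameMode.
; GetAttachPoint exposes the Arrow's world transform, likely for placing the next segment.
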(event OnComponentBeginOverlap(Box)
  (params (OverlappedComponent :type Primitive%20Component%20Object%20Reference) (OtherActor :type Actor%20Object%20Reference) (OtherComp :type Primitive%20Component%20Object%20Reference) (OtherBodyIndex :type Integer) (bFromSweep :type Boolean) (SweepResult :type Hit%20Result%20Structure%20%28by%20ref%29))
  (Utilities|Casting|CastToBP_Plaayer OtherActor)
  (bind _asbp_game_mode (Utilities|Casting|CastToBP_GameMode (Game|GetGameMode)))
  (Default|ExtendEnv _asbp_game_mode))

(event EventBeginPlay)

(event EventTick
  (params (DeltaSeconds :type Float%20%28single-precision%29)))

(fn ConstructionScript
  (CallFunction|SpawnEnv))

(fn GetAttachPoint
  (return (Transformation|GetWorldTransform (Variables|Default|GetArrow))))

(fn SpawnEnv
  (bind _sp6 (Variables|Default|Getsp6))
  (bind _sp7 (Variables|Default|Getsp7))
  (bind _sp2 (Variables|Default|Getsp2))
  (bind _sp3 (Variables|Default|Getsp3))
  (bind _returnvalue (Transformation|GetRelativeTransform _sp6))
  (bind _returnvalue_2 (Transformation|GetRelativeTransform _sp7))
  (bind _returnvalue_3 (Transformation|GetRelativeTransform _sp2))
  (bind _returnvalue_4 (Transformation|GetRelativeTransform _sp3))
  (Utilities|FlowControl|Sequence
    (:then_0
      (AddComponent|AddChildActorComponent false (Transformation|GetRelativeTransform (Variables|Default|Getsp4))))
    (:then_1
      (switch int (Math|Random|RandomIntegerinRange 0 6)
        (:0
          (AddComponent|AddChildActorComponent false _returnvalue_3))
        (:1
          (AddComponent|AddChildActorComponent false _returnvalue_3))
        (:2
          (AddComponent|AddChildActorComponent false _returnvalue_3))
        (:3
          (AddComponent|AddChildActorComponent false _returnvalue_3))
        (:4
          (AddComponent|AddChildActorComponent false _returnvalue_3))
        (:5
          (AddComponent|AddChildActorComponent false _returnvalue_3))
        (:6
          (AddComponent|AddChildActorComponent false _returnvalue_3))))
    (:then_2
      (switch int (Math|Random|RandomIntegerinRange 0 6)
        (:0
          (AddComponent|AddChildActorComponent false _returnvalue_4))
        (:1
          (AddComponent|AddChildActorComponent false _returnvalue_4))
        (:2
          (AddComponent|AddChildActorComponent false _returnvalue_4))
        (:3
          (AddComponent|AddChildActorComponent false _returnvalue_4))
        (:4
          (AddComponent|AddChildActorComponent false _returnvalue_4))
        (:5
          (AddComponent|AddChildActorComponent false _returnvalue_4))
        (:6
          (AddComponent|AddChildActorComponent false _returnvalue_4))))
    (:then_3
      (AddComponent|AddChildActorComponent false (Transformation|GetRelativeTransform (Variables|Default|Getsp8))))
    (:then_4
      (AddComponent|AddChildActorComponent false (Transformation|GetRelativeTransform (Variables|Default|Getsp1))))
    (:then_5
      (switch int (Math|Random|RandomIntegerinRange 0 6)
        (:0
          (AddComponent|AddChildActorComponent false _returnvalue))
        (:1
          (AddComponent|AddChildActorComponent false _returnvalue))
        (:2
          (AddComponent|AddChildActorComponent false _returnvalue))
        (:3
          (AddComponent|AddChildActorComponent false _returnvalue))
        (:4
          (AddComponent|AddChildActorComponent false _returnvalue))
        (:5
          (AddComponent|AddChildActorComponent false _returnvalue))
        (:6
          (AddComponent|AddChildActorComponent false _returnvalue))))
    (:then_6
      (switch int (Math|Random|RandomIntegerinRange 0 6)
        (:0
          (AddComponent|AddChildActorComponent false _returnvalue_2))
        (:1
          (AddComponent|AddChildActorComponent false _returnvalue_2))
        (:2
          (AddComponent|AddChildActorComponent false _returnvalue_2))
        (:3
          (AddComponent|AddChildActorComponent false _returnvalue_2))
        (:4
          (AddComponent|AddChildActorComponent false _returnvalue_2))
        (:5
          (AddComponent|AddChildActorComponent false _returnvalue_2))
        (:6
          (AddComponent|AddChildActorComponent false _returnvalue_2))))
    (:then_7
      (AddComponent|AddChildActorComponent false (Transformation|GetRelativeTransform (Variables|Default|Getsp5))))))