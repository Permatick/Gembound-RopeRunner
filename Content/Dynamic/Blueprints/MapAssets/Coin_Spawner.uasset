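; Coin spawner map asset that lays child actors, presumably coins, along one of two splines.
; The Construction Script reads the CoinJump flag from BP_GameMode to choose JumpSpline when set, otherwise Spline, and spawns nothing if the cast fails.
; It adds a manually attached child actor at each point's world-space location, looping from index 1 to the point count rather than from zero.
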(event EventBeginPlay)

(fn ConstructionScript
  (bind _spline (Variables|Default|GetSpline))
  (bind _jump_spline (Variables|Default|GetJump%20spline))
  (bind _asbp_game_mode (Utilities|Casting|CastToBP_GameMode (Game|GetGameMode)))
  (if (Variables|/Game/Dynamic/Blueprints/InputsAndGamemode/BP_GameMode.BP_GameMode_C|GetCoin%20Jump _asbp_game_mode)
    (for _index (range 1 (Spline|GetNumberOfSplinePoints _jump_spline))
      (AddComponent|AddChildActorComponent true (Math|Transform|MakeTransform (Spline|GetLocationatSplinePoint _jump_spline _index "World") "0, 0, 0" "1.000000,1.000000,1.000000")))
    (else
      (for _index_2 (range 1 (Spline|GetNumberOfSplinePoints _spline))
        (AddComponent|AddChildActorComponent true (Math|Transform|MakeTransform (Spline|GetLocationatSplinePoint _spline _index_2 "World") "0, 0, 0" "1.000000,1.000000,1.000000"))))))