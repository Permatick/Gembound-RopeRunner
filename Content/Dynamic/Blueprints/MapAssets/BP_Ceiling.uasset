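; Ceiling segment for a lane-based endless runner that exposes an arrow transform as the attach point.
; Its construction script builds lane spawn points from arrow components, then randomly adds child actors for obstacles, shootable obstacles and coins.
; When the rope character overlaps Box, it calls ExtendCeiling on the game mode and raises player walk speed by 4%.
; Any rope character overlapping the actor disables Box1 collision, regardless of PowerUp.
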(event OnComponentBeginOverlap(Box)
  (params (OverlappedComponent :type Primitive%20Component%20Object%20Reference) (OtherActor :type Actor%20Object%20Reference) (OtherComp :type Primitive%20Component%20Object%20Reference) (OtherBodyIndex :type Integer) (bFromSweep :type Boolean) (SweepResult :type Hit%20Result%20Structure%20%28by%20ref%29))
  (Utilities|Casting|CastToBP_RopeCharacter OtherActor)
  (bind _asbp_rope_game_mode (Utilities|Casting|CastToBP_RopeGameMode (Game|GetGameMode)))
  (Default|ExtendCeiling _asbp_rope_game_mode)
  (bind _asbp_rope_character (Utilities|Casting|CastToBP_RopeCharacter (Game|GetPlayerCharacter 0)))
  (Variables|/Script/Engine.CharacterMovementComponent|SetMaxWalkSpeed (Variables|/Script/Engine.Character|GetCharacterMovement _asbp_rope_character) (* (Variables|/Script/Engine.CharacterMovementComponent|GetMaxWalkSpeed (Variables|/Script/Engine.Character|GetCharacterMovement _asbp_rope_character)) 1.04))
  (Development|PrintString (Utilities|String|ToString(Vector) (Transformation|GetVelocity _asbp_rope_character))))

(event OnComponentBeginOverlap(Box1)
  (params (OverlappedComponent :type Primitive%20Component%20Object%20Reference) (OtherActor :type Actor%20Object%20Reference) (OtherComp :type Primitive%20Component%20Object%20Reference) (OtherBodyIndex :type Integer) (bFromSweep :type Boolean) (SweepResult :type Hit%20Result%20Structure%20%28by%20ref%29)))

(event Collision|EventActorBeginOverlap
  (params (OtherActor :type Actor%20Object%20Reference))
  (bind _box1 (Variables|Default|GetBox1))
  (bind _asbp_rope_character (Utilities|Casting|CastToBP_RopeCharacter OtherActor))
  (if (Variables|/Game/Dynamic/Blueprints/Characters/BP_Character/BP_RopeCharacter.BP_RopeCharacter_C|GetPowerUp _asbp_rope_character)
    (Collision|SetCollisionEnabled _box1 "NoCollision")
    (else
      (Collision|SetCollisionEnabled _box1 "NoCollision"))))

(fn ConstructionScript
  (CallFunction|ObstacleSpawnCeiling)
  (CallFunction|ObstacleSpawnPointCeiling)
  (CallFunction|VurulabilenObstacleSpawnPointCeiling)
  (CallFunction|SpawnVurulabilenObstaclesCeiling)
  (CallFunction|CoinSpawnPoint1)
  (CallFunction|SpawnCoins1))

(fn GetCeilingAttachPoint
  (return (Transformation|GetWorldTransform (Variables|Default|GetArrow))))

(fn CoinSpawnPoint1
  (for _array_element (Variables|Default|GetLane%20Position)
    (for _index (range 0 9)
      (bind _returnvalue (AddComponent|AddArrowComponent false (Math|Transform|MakeTransform (Math|Vector|MakeVector (Math|Conversions|ToFloat(Integer) (* _index 75)) _array_element -8e+02))))
      (Components|Arrow|SetArrowColor(LinearColor) _returnvalue "(R=0.246839,G=0.182225,B=1.000000,A=1.000000)")
      (Utilities|Array|Add (Variables|Default|GetCoin%20Spawn) (Transformation|GetWorldTransform _returnvalue)))))

(fn SpawnCoins1
  (bind _output_get (Variables|Default|SetRandom%20Spawn%20Points (Variables|Default|GetCoin%20Spawn)))
  (Utilities|Array|Shuffle _output_get)
  (for _index (range 0 (Math|Random|RandomIntegerinRange 5 8))
    (switch int 0
      (:0
        (AddComponent|AddChildActorComponent false (Math|Transform|MakeRelativeTransform (Utilities|Array|Get(acopy) (Variables|Default|GetRandom%20Spawn%20Points) _index) (Transformation|GetActorTransform)))))))

(fn ObstacleSpawnPointCeiling
  (Variables|Default|SetRandom%20Spawn%20Points (Variables|Default|GetSpawn%20Points))
  (bind _index (Utilities|FlowControl|ForLoopwithBreak 0 (Math|Random|RandomIntegerinRange 0 2))
    (:LoopBody
      (Utilities|Array|RemoveIndex (Variables|Default|GetRandom%20Spawn%20Points) _index)
      (switch int (Math|Random|RandomIntegerinRange 0 2)
        (:0
          (AddComponent|AddChildActorComponent false (Math|Transform|MakeRelativeTransform (Utilities|Array|Get(acopy) (Variables|Default|GetRandom%20Spawn%20Points) _index) (Transformation|GetActorTransform))))
        (:1
          (AddComponent|AddChildActorComponent false (Math|Transform|MakeRelativeTransform (Utilities|Array|Get(acopy) (Variables|Default|GetRandom%20Spawn%20Points) _index) (Transformation|GetActorTransform))))
        (:2
          (AddComponent|AddChildActorComponent false (Math|Transform|MakeRelativeTransform (Utilities|Array|Get(acopy) (Variables|Default|GetRandom%20Spawn%20Points) _index) (Transformation|GetActorTransform))))))))

(fn ObstacleSpawnCeiling
  (for _array_element (Variables|Default|GetLane%20Position)
    (for _index (range 0 1)
      (bind _returnvalue (AddComponent|AddArrowComponent false (Math|Transform|MakeTransform (Math|Vector|MakeVector 0.0 _array_element -8e+02))))
      (Utilities|Array|Add (Variables|Default|GetSpawn%20Points) (Transformation|GetWorldTransform _returnvalue)))))

(fn VurulabilenObstacleSpawnPointCeiling
  (for _array_element (Variables|Default|GetLane%20Position)
    (for _index (range 0 9)
      (bind _returnvalue (AddComponent|AddArrowComponent false (Math|Transform|MakeTransform (Math|Vector|MakeVector (Math|Conversions|ToFloat(Integer) (* _index 75)) _array_element 0.0))))
      (Components|Arrow|SetArrowColor(LinearColor) _returnvalue "(R=0.246839,G=0.182225,B=1.000000,A=1.000000)")
      (Utilities|Array|Add (Variables|Default|GetSpawn%20Points) (Transformation|GetWorldTransform _returnvalue)))))

(fn SpawnVurulabilenObstaclesCeiling
  (bind _returnvalue (Math|Random|RandomIntegerinRange 0 2))
  (bind _output_get (Variables|Default|SetRandom%20Spawn%20Points (Variables|Default|GetSpawn%20Points)))
  (Utilities|Array|Shuffle _output_get)
  (if (not (== _returnvalue 1))
    (for _index (range 0 _returnvalue)
      (switch int (Math|Random|RandomIntegerinRange 0 1)
        (:0
          (AddComponent|AddChildActorComponent false (Math|Transform|MakeRelativeTransform (Utilities|Array|Get(acopy) (Variables|Default|GetRandom%20Spawn%20Points) _index) (Transformation|GetActorTransform))))))))