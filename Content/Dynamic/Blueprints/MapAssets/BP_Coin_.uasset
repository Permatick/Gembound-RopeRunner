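; BP_Coin_ is a collectible coin that works for both BP_Plaayer and BP_RopeCharacter, incrementing the matching game mode's counter and refreshing the character's coin count.
; Sphere1 overlaps collect the coin and also destroy any overlapping BP_SlidingObstacle.
; When a powered-up rope character enters CollectMagnet, the Magnet timeline interpolates the coin toward a velocity-led point below the player.
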(event OnComponentBeginOverlap(CollectMagnet)
  (params (OverlappedComponent :type Primitive%20Component%20Object%20Reference) (OtherActor :type Actor%20Object%20Reference) (OtherComp :type Primitive%20Component%20Object%20Reference) (OtherBodyIndex :type Integer) (bFromSweep :type Boolean) (SweepResult :type Hit%20Result%20Structure%20%28by%20ref%29))
  (bind _returnvalue (Game|GetPlayerCharacter 0))
  (bind _returnvalue_2 (Transformation|GetActorLocation _returnvalue))
  (bind _asbp_rope_character (Utilities|Casting|CastToBP_RopeCharacter OtherActor))
  (if (Variables|/Game/Dynamic/Blueprints/Characters/BP_Character/BP_RopeCharacter.BP_RopeCharacter_C|GetPowerUp _asbp_rope_character)
    (bind _slide (Timeline|Magnet PlayFromStart)
      (:Update
        (Transformation|SetActorLocation (+ _slide (Math|Interpolation|VInterpTo (.location (Transformation|GetActorTransform)) (Math|Vector|MakeVector (+ (.x _returnvalue_2) (/ (.x (Transformation|GetVelocity _returnvalue)) 8.0)) (.y _returnvalue_2) (- (.z _returnvalue_2) 1.5e+02)) (Utilities|Time|GetWorldDeltaSeconds) 1e+01)) false false)))))

(event OnComponentBeginOverlap(Sphere1)
  (params (OverlappedComponent :type Primitive%20Component%20Object%20Reference) (OtherActor :type Actor%20Object%20Reference) (OtherComp :type Primitive%20Component%20Object%20Reference) (OtherBodyIndex :type Integer) (bFromSweep :type Boolean) (SweepResult :type Hit%20Result%20Structure%20%28by%20ref%29))
  (Utilities|FlowControl|Sequence
    (:then_0
      (bind _asbp_sliding_obstacle (Utilities|Casting|CastToBP_SlidingObstacle OtherActor))
      (Actor|DestroyActor _asbp_sliding_obstacle))
    (:then_2
      (bind _asbp_plaayer (Utilities|Casting|CastToBP_Plaayer OtherActor))
      (bind _asbp_game_mode (Utilities|Casting|CastToBP_GameMode (Game|GetGameMode)))
      (bind _result (Math|Integer|IncrementInt (Variables|/Game/Dynamic/Blueprints/InputsAndGamemode/BP_GameMode.BP_GameMode_C|GetCoins _asbp_game_mode))
        (:%20%20
          (Actor|DestroyActor)
          (Default|UpdateCoins _asbp_plaayer))))
    (:then_3
      (CallFunction|CollectRopeCoin OtherActor))))

(fn ConstructionScript)

(fn CollectRopeCoin
  (params (Actor :type Actor%20Object%20Reference))
  (bind _asbp_rope_character (Utilities|Casting|CastToBP_RopeCharacter Actor))
  (bind _asbp_rope_game_mode (Utilities|Casting|CastToBP_RopeGameMode (Game|GetGameMode)))
  (bind _result (Math|Integer|IncrementInt (Variables|/Game/Dynamic/Blueprints/InputsAndGamemode/BP_RopeGameMode.BP_RopeGameMode_C|Getcoins%201 _asbp_rope_game_mode))
    (:%20%20
      (Actor|DestroyActor)
      (Default|UpdateCoinsRope _asbp_rope_character))))