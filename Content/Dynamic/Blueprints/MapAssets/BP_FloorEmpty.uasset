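; BP_FloorEmpty is an endless-runner floor tile that populates its lanes with random child actors and chains into the next tile.
; Construction builds spawn points from lane offsets, then randomly adds coins, another child actor or nothing.
; Its one-shot Box overlap makes BP_GameMode extend the floor, adds points, raises player speed until MaxSpeed, then, after a delay, removes old floor and environment pieces.
; Cube1 flags overlapping BP_Blocks as colliding.
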(event OnComponentBeginOverlap(Box)
  (params (OverlappedComponent :type Primitive%20Component%20Object%20Reference) (OtherActor :type Actor%20Object%20Reference) (OtherComp :type Primitive%20Component%20Object%20Reference) (OtherBodyIndex :type Integer) (bFromSweep :type Boolean) (SweepResult :type Hit%20Result%20Structure%20%28by%20ref%29))
  (Utilities|FlowControl|DoOnce false
    (:Completed
      (bind _asbp_game_mode (Utilities|Casting|CastToBP_GameMode (Game|GetGameMode)))
      (Default|ExtendFloor _asbp_game_mode)
      (bind _asbp_plaayer (Utilities|Casting|CastToBP_Plaayer (Game|GetPlayerCharacter 0)))
      (if (Variables|/Game/Dynamic/Blueprints/InputsAndGamemode/BP_GameMode.BP_GameMode_C|GetMaxSpeed _asbp_game_mode)
        _
        (else
          (Variables|/Game/Dynamic/Blueprints/Characters/BP_Character/BP_Plaayer.BP_Plaayer_C|SetSpeed _asbp_plaayer (+ 2e+01 (Variables|/Game/Dynamic/Blueprints/Characters/BP_Character/BP_Plaayer.BP_Plaayer_C|GetSpeed _asbp_plaayer)))))
      (bind _asbp_game_mode_2 (Utilities|Casting|CastToBP_GameMode (Game|GetGameMode)))
      (Variables|/Game/Dynamic/Blueprints/InputsAndGamemode/BP_GameMode.BP_GameMode_C|SetCurrent%20Point%20Floor _asbp_game_mode_2 (+ (Variables|/Game/Dynamic/Blueprints/InputsAndGamemode/BP_GameMode.BP_GameMode_C|GetPoints%20Multi _asbp_game_mode_2) (Variables|/Game/Dynamic/Blueprints/InputsAndGamemode/BP_GameMode.BP_GameMode_C|GetCurrent%20Point%20Floor _asbp_game_mode_2)))
      (Utilities|FlowControl|Delay 0.731)
      (Actor|DestroyActor)
      (Utilities|Array|RemoveItem (Variables|/Game/Dynamic/Blueprints/InputsAndGamemode/BP_GameMode.BP_GameMode_C|GetFloorTiles_0 _asbp_game_mode_2) (Utilities|Array|Get(acopy) (Variables|/Game/Dynamic/Blueprints/InputsAndGamemode/BP_GameMode.BP_GameMode_C|GetFloorTiles_0 _asbp_game_mode_2)))
      (Actor|DestroyActor (Utilities|Array|Get(acopy) (Variables|/Game/Dynamic/Blueprints/InputsAndGamemode/BP_GameMode.BP_GameMode_C|GetBP%20Env _asbp_game_mode_2)))
      (Utilities|Array|RemoveItem (Variables|/Game/Dynamic/Blueprints/InputsAndGamemode/BP_GameMode.BP_GameMode_C|GetBP%20Env _asbp_game_mode_2) (Utilities|Array|Get(acopy) (Variables|/Game/Dynamic/Blueprints/InputsAndGamemode/BP_GameMode.BP_GameMode_C|GetBP%20Env _asbp_game_mode_2))))))

(event OnComponentBeginOverlap(Cube1)
  (params (OverlappedComponent :type Primitive%20Component%20Object%20Reference) (OtherActor :type Actor%20Object%20Reference) (OtherComp :type Primitive%20Component%20Object%20Reference) (OtherBodyIndex :type Integer) (bFromSweep :type Boolean) (SweepResult :type Hit%20Result%20Structure%20%28by%20ref%29))
  (bind _asbp_block (Utilities|Casting|CastToBP_Block OtherActor))
  (Variables|/Game/Dynamic/Blueprints/Enemy/BP_Block.BP_Block_C|SetCollission _asbp_block true))

(event EventBeginPlay)

(event EventTick
  (params (DeltaSeconds :type Float%20%28single-precision%29)))

(fn ConstructionScript
  (CallFunction|ObstacleSpawn)
  (CallFunction|SpawnObstacles))

(fn GetAttachPoint
  (return (Transformation|GetWorldTransform (Variables|Default|GetArrow))))

(fn ObstacleSpawn
  (for _array_element (Variables|Default|GetLane%20Position)
    (for _index (range 0 1)
      (bind _returnvalue (AddComponent|AddArrowComponent false (Math|Transform|MakeTransform (Math|Vector|MakeVector 0.0 _array_element 0.0))))
      (Utilities|Array|Add (Variables|Default|GetSpawn%20Points) (Transformation|GetWorldTransform _returnvalue)))))

(fn SpawnCoins
  (params (Coins%20Transform%20 :type Transform))
  (AddComponent|AddChildActorComponent false Coins%20Transform%20))

(fn SpawnObstacles
  (bind _output_get (LocalVariables|Setrandom%20spawn%20points (Variables|Default|GetSpawn%20Points)))
  (for (_ _array_index) _output_get
    (Utilities|Array|RemoveIndex _output_get _array_index)
    (switch int (Math|Random|RandomIntegerinRange 0 5)
      (:0
        (CallFunction|SpawnCoins (Math|Transform|MakeRelativeTransform (Utilities|Array|Get(acopy) (LocalVariables|GetRandom%20Spawn%20Points) _array_index) (Transformation|GetActorTransform)) :!label _label))
      (:1
        (AddComponent|AddChildActorComponent false (Math|Transform|MakeRelativeTransform (Utilities|Array|Get(acopy) (LocalVariables|GetRandom%20Spawn%20Points) _array_index) (Transformation|GetActorTransform))))
      (:2
        (goto _label)))))