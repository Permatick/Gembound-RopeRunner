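; BP_ActiveObject is an enemy pawn that walks along its forward vector and kills player characters on contact.
; A Walk event feeds scaled movement input, with no caller in this file.
; Actor overlap calls Dead on BP_RopeCharacter, while Box2 overlap does so on BP_Plaayer.
; When anything stops overlapping Box or Box1, Turn rotates the actor 180 degrees, suggesting ledge-detection patrolling.
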(event OnComponentBeginOverlap(Box2)
  (params (OverlappedComponent :type Primitive%20Component%20Object%20Reference) (OtherActor :type Actor%20Object%20Reference) (OtherComp :type Primitive%20Component%20Object%20Reference) (OtherBodyIndex :type Integer) (bFromSweep :type Boolean) (SweepResult :type Hit%20Result%20Structure%20%28by%20ref%29))
  (bind _asbp_plaayer (Utilities|Casting|CastToBP_Plaayer OtherActor))
  (Default|Dead _asbp_plaayer))

(event OnComponentEndOverlap(Box)
  (params (OverlappedComponent :type Primitive%20Component%20Object%20Reference) (OtherActor :type Actor%20Object%20Reference) (OtherComp :type Primitive%20Component%20Object%20Reference) (OtherBodyIndex :type Integer))
  (CallFunction|Turn))

(event OnComponentEndOverlap(Box1)
  (params (OverlappedComponent :type Primitive%20Component%20Object%20Reference) (OtherActor :type Actor%20Object%20Reference) (OtherComp :type Primitive%20Component%20Object%20Reference) (OtherBodyIndex :type Integer))
  (CallFunction|Turn))

(event Custom|Walk
  (params (ScaleValue :type Float%20%28single-precision%29))
  (Pawn|Input|AddMovementInput (Transformation|GetActorForwardVector) ScaleValue false))

(event EventBeginPlay)

(event EventTick
  (params (DeltaSeconds :type Float%20%28single-precision%29)))

(event Collision|EventActorBeginOverlap
  (params (OtherActor :type Actor%20Object%20Reference))
  (bind _asbp_rope_character (Utilities|Casting|CastToBP_RopeCharacter OtherActor))
  (Default|Dead _asbp_rope_character))

(fn ConstructionScript)

(fn Turn
  (Transformation|SetActorRotation (Math|Rotator|CombineRotators (Transformation|GetActorRotation) "0.000000,180.000000,0.000000")))