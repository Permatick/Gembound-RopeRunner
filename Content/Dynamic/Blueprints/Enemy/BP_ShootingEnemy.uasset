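; BP_ShootingEnemy is an enemy that shoots at player characters derived from BP_BaseCharacter when it sees them.
; Each PawnSensing sighting snaps its rotation toward the character and spawns a BP_EnemyProjectile at the Projectile component's world transform.
; Overlapping its Box component instantly destroys the character.
; All logic is event-driven, with no Tick logic or explicit fire-rate control.
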(event OnSeePawn(PawnSensing)
  (params (Pawn :type Pawn%20Object%20Reference))
  (bind _asbp_base_character (Utilities|Casting|CastToBP_BaseCharacter Pawn))
  (Transformation|SetActorRotation (Math|Rotator|FindRelativeLookatRotation (Math|Conversions|ToTransform(Vector) (Transformation|GetActorLocation)) (Transformation|GetActorLocation _asbp_base_character)))
  (Game|SpawnActorfromClass "/Game/Dynamic/Blueprints/Enemy/BP_EnemyProjectile.BP_EnemyProjectile_C" (Transformation|GetWorldTransform (Variables|Default|GetProjectile)) "Undefined" "MultiplyWithRoot" 0 0))

(event OnComponentBeginOverlap(Box)
  (params (OverlappedComponent :type Primitive%20Component%20Object%20Reference) (OtherActor :type Actor%20Object%20Reference) (OtherComp :type Primitive%20Component%20Object%20Reference) (OtherBodyIndex :type Integer) (bFromSweep :type Boolean) (SweepResult :type Hit%20Result%20Structure%20%28by%20ref%29))
  (bind _asbp_base_character (Utilities|Casting|CastToBP_BaseCharacter OtherActor))
  (Actor|DestroyActor _asbp_base_character))

(event EventBeginPlay)

(event Collision|EventActorBeginOverlap
  (params (OtherActor :type Actor%20Object%20Reference)))

(event EventTick
  (params (DeltaSeconds :type Float%20%28single-precision%29)))

(fn ConstructionScript)

(fn NewFunction)