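; BP_Moveable_Obstacle is a hazard that advances along negative world X and kills the rope character on contact.
; Each Tick, a large box trace biased toward negative X checks for a specific object type.
; While it gets a hit, the actor steps a fixed distance per frame, independent of delta time.
; Overlapping a BP_RopeCharacter calls that character's Dead function.
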(event EventBeginPlay)

(event Collision|EventActorBeginOverlap
  (params (OtherActor :type Actor%20Object%20Reference))
  (bind _asbp_rope_character (Utilities|Casting|CastToBP_RopeCharacter OtherActor))
  (Default|Dead _asbp_rope_character))

(event EventTick
  (params (DeltaSeconds :type Float%20%28single-precision%29))
  (bind _returnvalue (Transformation|GetActorLocation))
  (bind _returnvalue_2 (Class|KismetSystemLibrary|BoxTraceSingleforObjects (Math|Vector|MakeVector (- (.x _returnvalue) 2.5e+03) (.y _returnvalue) (+ (.z _returnvalue) 2e+02)) (Transformation|GetActorLocation) "5000.000000,700.000000,500.000000" "0, 0, 0" (Utilities|Array|MakeArray "ObjectTypeQuery9") false 0 "None" true))
  (if _returnvalue_2
    (Transformation|SetActorLocation (Math|Vector|MakeVector (- (.x _returnvalue) 15.0) (.y _returnvalue) (.z _returnvalue)) false false)))

(fn ConstructionScript)