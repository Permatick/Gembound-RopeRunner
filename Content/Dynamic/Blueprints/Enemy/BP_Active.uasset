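; BP_Active is a moving enemy hazard that kills the player's BP_RopeCharacter on contact.
; On BeginPlay it caches its spawn location and plays a timeline whose track is added to that location each update to move the actor without sweeping.
; Overlaps on either the actor or its Box component cast to BP_RopeCharacter and call Dead.
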(event OnComponentBeginOverlap(Box)
  (params (OverlappedComponent :type Primitive%20Component%20Object%20Reference) (OtherActor :type Actor%20Object%20Reference) (OtherComp :type Primitive%20Component%20Object%20Reference) (OtherBodyIndex :type Integer) (bFromSweep :type Boolean) (SweepResult :type Hit%20Result%20Structure%20%28by%20ref%29))
  (bind _asbp_rope_character (Utilities|Casting|CastToBP_RopeCharacter OtherActor))
  (Default|Dead _asbp_rope_character))

(event EventBeginPlay
  (bind _output_get (Variables|Default|SetNewVar (Transformation|GetActorLocation)))
  (bind _newtrack_0 (Timeline|Zaman%20Çizelgesi PlayFromStart)
    (:Update
      (Transformation|SetActorLocation (+ _output_get _newtrack_0) false false))))

(event Collision|EventActorBeginOverlap
  (params (OtherActor :type Actor%20Object%20Reference))
  (bind _asbp_rope_character (Utilities|Casting|CastToBP_RopeCharacter OtherActor))
  (Default|Dead _asbp_rope_character))

(event EventTick
  (params (DeltaSeconds :type Float%20%28single-precision%29)))

(fn ConstructionScript)