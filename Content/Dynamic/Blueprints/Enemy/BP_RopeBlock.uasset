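; Falling block hazard that kills a BP_RopeCharacter overlapping the actor or a BP_Plaayer overlapping its Box.
; On BeginPlay a one-in-ten roll starts a looping timer that box-traces a wide, thin slab at the block's position for one custom object type.
; A hit latches Fall, and Tick, throttled by a short Delay, then steps the block straight down with sweep.
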(event OnComponentBeginOverlap(Box)
  (params (OverlappedComponent :type Primitive%20Component%20Object%20Reference) (OtherActor :type Actor%20Object%20Reference) (OtherComp :type Primitive%20Component%20Object%20Reference) (OtherBodyIndex :type Integer) (bFromSweep :type Boolean) (SweepResult :type Hit%20Result%20Structure%20%28by%20ref%29))
  (bind _asbp_plaayer (Utilities|Casting|CastToBP_Plaayer OtherActor))
  (Default|Dead _asbp_plaayer))

(event Custom|CustomEvent
  (bind _returnvalue (Transformation|GetActorLocation))
  (bind _returnvalue_2 (Class|KismetSystemLibrary|BoxTraceSingleforObjects _returnvalue _returnvalue "3031.000000,700.000000,10.000000" "0, 0, 0" (Utilities|Array|MakeArray "ObjectTypeQuery9") false 0 "None" true))
  (if _returnvalue_2
    (Variables|Default|Setfall true)))

(event EventBeginPlay
  (if (== (Math|Random|RandomIntegerinRange 0 9) 0)
    (Utilities|Time|SetTimerbyEvent (delegate Custom|CustomEvent) 0.231 true)))

(event Collision|EventActorBeginOverlap
  (params (OtherActor :type Actor%20Object%20Reference))
  (bind _asbp_rope_character (Utilities|Casting|CastToBP_RopeCharacter OtherActor))
  (Default|Dead _asbp_rope_character))

(event EventTick
  (params (DeltaSeconds :type Float%20%28single-precision%29))
  (bind _returnvalue (Transformation|GetActorLocation))
  (Utilities|FlowControl|Delay 0.0431)
  (if (Variables|Default|Getfall)
    (Transformation|SetActorLocation (Math|Vector|MakeVector (.x _returnvalue) (.y _returnvalue) (- (.z _returnvalue) 1e+02)) true false)))

(fn ConstructionScript)