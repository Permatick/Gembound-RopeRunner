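; BP_RopeGameMode is the game mode for a rope level, managing a chained run of ceiling tiles.
; BeginPlay spawns the initial BP_Ceiling tiles, each at the previous tile's attach point, and reads saved coins from the "coin" slot inside that same loop.
; ExtendCeiling adds a tile and destroys the oldest once the count exceeds NumberOfTiles + 1, keeping a rolling window; nothing in this graph calls it.
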(event EventBeginPlay
  (for _index (range 0 (- (Variables|Default|GetNumber%20Of%20Tiles) 2))
    (CallFunction|AddCeiling)
    (bind _returnvalue (SaveGame|LoadGamefromSlot "coin"))
    (bind _asbp_save_game (Utilities|Casting|CastToBP_SaveGame _returnvalue))
    (Variables|Default|Setcoins%201 (Variables|/Game/Dynamic/Blueprints/InputsAndGamemode/BP_SaveGame.BP_SaveGame_C|GetCoin _asbp_save_game))))

(event EventTick
  (params (DeltaSeconds :type Float%20%28single-precision%29)))

(fn ConstructionScript)

(fn AddCeiling
  (bind _returnvalue (Game|SpawnActorfromClass "/Game/Dynamic/Blueprints/MapAssets/BP_Ceiling.BP_Ceiling_C" (Variables|Default|GetCeiling%20Attach%20Point) "Undefined" "MultiplyWithRoot" 0 0))
  (bind _returnvalue_2 (Default|GetCeilingAttachPoint _returnvalue))
  (Variables|Default|SetCeiling%20Attach%20Point _returnvalue_2)
  (Utilities|Array|Add (Variables|Default|GetCeiling%20Tiles) _returnvalue))

(fn ExtendCeiling
  (bind _ceiling_tiles (Variables|Default|GetCeiling%20Tiles))
  (bind _output (Utilities|Array|Get(acopy) _ceiling_tiles))
  (CallFunction|AddCeiling)
  (if (> (Utilities|Array|Length (Variables|Default|GetCeiling%20Tiles)) (+ (Variables|Default|GetNumber%20Of%20Tiles) 1))
    (Actor|DestroyActor _output)
    (Utilities|Array|RemoveItem _ceiling_tiles _output)))