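; Game mode that builds an endlessly extendable track of floor and environment tiles, consistent with an endless runner.
; Each tile spawns at the previous tile's attach point; Extend functions append one and destroy the oldest beyond a cap.
; BeginPlay lays initial tiles, reloads coin, point and timer saves inside the floor loop, starts music and briefly sets the player's MapON.
; Key 9 opens Rope_Map.
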(event EventBeginPlay
  (Utilities|FlowControl|Sequence
    (:then_0
      (Input|SetInputModeGameOnly (Game|GetPlayerController 0) false)
      (for _index (range 0 (- (Variables|Default|GetNumber%20Of%20Tiles) 2))
        (CallFunction|AddFloor)
        (bind _returnvalue (SaveGame|LoadGamefromSlot "Coin"))
        (bind _asbp_save_game (Utilities|Casting|CastToBP_SaveGame _returnvalue))
        (Variables|Default|SetCoins (Variables|/Game/Dynamic/Blueprints/InputsAndGamemode/BP_SaveGame.BP_SaveGame_C|GetCoin _asbp_save_game))
        (bind _returnvalue_2 (SaveGame|LoadGamefromSlot "Current Point"))
        (bind _asbp_save_game_2 (Utilities|Casting|CastToBP_SaveGame _returnvalue_2))
        (Variables|Default|SetCurrent%20Point (Variables|/Game/Dynamic/Blueprints/InputsAndGamemode/BP_SaveGame.BP_SaveGame_C|GetCurrent%20Point _asbp_save_game_2))
        (bind _returnvalue_3 (SaveGame|LoadGamefromSlot "MusicTimer"))
        (bind _asbp_save_game_3 (Utilities|Casting|CastToBP_SaveGame _returnvalue_3))
        (Variables|Default|SetCurrent%20Time (Variables|/Game/Dynamic/Blueprints/InputsAndGamemode/BP_SaveGame.BP_SaveGame_C|GetTimer _asbp_save_game_3))))
    (:then_1
      (for _index_2 (range 0 16)
        (CallFunction|AddEnv)))
    (:then_2
      (bind _asgame_instance_music (Utilities|Casting|CastToGameInstance_Music (Game|GetGameInstance)))
      (Default|PlayMusic _asgame_instance_music))
    (:then_3
      (bind _asbp_plaayer (Utilities|Casting|CastToBP_Plaayer (Game|GetPlayerCharacter 0)))
      (Variables|/Game/Dynamic/Blueprints/Characters/BP_Character/BP_Plaayer.BP_Plaayer_C|SetMapON _asbp_plaayer true)
      (Utilities|FlowControl|Delay 1.0)
      (Variables|/Game/Dynamic/Blueprints/Characters/BP_Character/BP_Plaayer.BP_Plaayer_C|SetMapON _asbp_plaayer false))))

(event EventTick
  (params (DeltaSeconds :type Float%20%28single-precision%29)))

(event Input|KeyboardEvents|9
  (params (Key :type Key%20Structure :default "None"))
  (:Pressed
    (Game|OpenLevel(byObjectReference) "/Game/Dynamic/Map/Rope_Map.Rope_Map")))

(fn ConstructionScript)

(fn AddFloor
  (bind _returnvalue (Game|SpawnActorfromClass "/Game/Dynamic/Blueprints/MapAssets/BP_Floor.BP_Floor_C" (Variables|Default|GetFloor%20Attach%20Point) "Undefined" "MultiplyWithRoot" 0 0))
  (bind _returnvalue_2 (Default|GetAttachPoint _returnvalue))
  (Variables|Default|SetFloor%20Attach%20Point _returnvalue_2)
  (Utilities|Array|Add (Variables|Default|GetFloorTiles) _returnvalue))

(fn ExtendFloor
  (bind _floortiles (Variables|Default|GetFloorTiles))
  (bind _output (Utilities|Array|Get(acopy) _floortiles))
  (CallFunction|AddFloor)
  (if (> (Utilities|Array|Length (Variables|Default|GetFloorTiles)) (+ (Variables|Default|GetNumber%20Of%20Tiles) 1))
    (Actor|DestroyActor _output)
    (Utilities|Array|RemoveItem _floortiles _output)))

(fn AddEnv
  (bind _returnvalue (Game|SpawnActorfromClass "/Game/Dynamic/Blueprints/MapAssets/BP_Enviornment.BP_Enviornment_C" (Variables|Default|GetBuilding%20Spawn%20Point) "Undefined" "MultiplyWithRoot" 0 0))
  (bind _returnvalue_2 (Default|GetAttachPoint _returnvalue))
  (Variables|Default|SetBuilding%20Spawn%20Point _returnvalue_2)
  (Utilities|Array|Add (Variables|Default|GetBP%20Env) _returnvalue))

(fn ExtendEnv
  (bind _bp_env (Variables|Default|GetBP%20Env))
  (bind _output (Utilities|Array|Get(acopy) _bp_env))
  (CallFunction|AddEnv)
  (if (> (Utilities|Array|Length (Variables|Default|GetBP%20Env)) 31)
    (Actor|DestroyActor _output)
    (Utilities|Array|RemoveItem _bp_env _output)))