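; Game mode that builds and recycles a chain of BP_Floor tiles, forming a continuously extendable track.
; On BeginPlay it spawns TileNumber tiles through FloorMaker, which places each at the stored spawn transform and then updates it from that tile's BirleşmeNoktası (join point).
; FloorExtender adds a tile and destroys the oldest once the FloorTile array exceeds TileNumber plus two, keeping the live tile count bounded.
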(event EventBeginPlay
  (for _index (range 0 (- (Variables|Default|GetTile%20Number) 1))
    (CallFunction|FloorMaker)))

(event EventTick
  (params (DeltaSeconds :type Float%20%28single-precision%29)))

(fn ConstructionScript)

(fn FloorMaker
  (bind _returnvalue (Game|SpawnActorfromClass "/Game/Dynamic/Blueprints/Assets/BP_Floor.BP_Floor_C" (Variables|Default|GetFloor%20Make%20Point) "Undefined" "MultiplyWithRoot" 0 0))
  (bind _returnvalue_2 (Default|BirleşmeNoktası _returnvalue))
  (Variables|Default|SetFloor%20Make%20Point _returnvalue_2)
  (Utilities|Array|Add (Variables|Default|GetFloorTile) _returnvalue))

(fn FloorExtender
  (bind _floortile (Variables|Default|GetFloorTile))
  (bind _output (Utilities|Array|Get(acopy) _floortile))
  (CallFunction|FloorMaker)
  (if (> (Utilities|Array|Length (Variables|Default|GetFloorTile)) (+ (Variables|Default|GetTile%20Number) 2))
    (Actor|DestroyActor _output)
    (Utilities|Array|RemoveItem _floortile _output)))